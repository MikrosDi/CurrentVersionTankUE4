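; Enemy turret Blueprint that manages the floating health bar above the turret.
; On BeginPlay it hands itself to the W_HpBar_EnemyTurret widget and caches the player's BP_TankPawn.
; Each Tick it turns the widget toward the player's camera using only X and Y positions, and destroys it once HealthComponent reaches zero health.
; A leftover FireAnyway call is unwired and never runs.
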(event EventBeginPlay
  (bind _asw_hp_bar_enemy_turret (Utilities|Casting|CastToW_HpBar_EnemyTurret (UserInterface|GetUserWidgetObject (Variables|Default|GetWidget%20Health))))
  (Variables|/Game/Widgets/HP/W_HpBar_EnemyTurret.W_HpBar_EnemyTurret_C|SetEnemyTurret _asw_hp_bar_enemy_turret self)
  (bind _asbp_tank_pawn (Utilities|Casting|CastToBP_TankPawn (Game|Player|GetPlayerPawn 0)))
  (Variables|Default|SetPlayer _asbp_tank_pawn))

(event Collision|EventActorBeginOverlap
  (params (OtherActor :type Actor%20Object%20Reference)))

(event EventTick
  (params (DeltaSeconds :type Float%20%28single-precision%29))
  (bind _widget_health (Variables|Default|GetWidget%20Health))
  (bind _player (Variables|Default|GetPlayer))
  (bind _returnvalue (Transformation|GetWorldLocation _widget_health))
  (bind _cameracomponent (Variables|/Script/TankProject.TankPawn|GetCameraComponent _player))
  (bind _returnvalue_2 (Transformation|GetWorldLocation _cameracomponent))
  (if (Utilities|IsValid (Variables|Default|GetWidget%20Health))
    (Transformation|SetWorldRotation _widget_health (Math|Rotator|FindLookatRotation (Math|Vector|MakeVector (.x _returnvalue) (.y _returnvalue) 0.0) (Math|Vector|MakeVector (.x _returnvalue_2) (.y _returnvalue_2) 0.0)) false false)
    (if (== (Variables|/Script/TankProject.HealthComponent|GetCurrentHealth (Variables|Default|GetHealthComponent)) 0.0)
      (Components|DestroyComponent (Variables|Default|GetWidget%20Health)))))

(fn ConstructionScript)